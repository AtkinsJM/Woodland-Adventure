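; BP_AnimalPlayerController is a player controller that lets the player switch control between animal characters with the number keys.
; Keys 1 to 4 map to the fox, pig, doe and stag Blueprints.
; Each press finds all actors of that class in the level and possesses the first one, doing nothing if none exist.
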(event EventBeginPlay)

(event EventTick
  (params (DeltaSeconds :type Float%20%28single-precision%29)))

(event Input|KeyboardEvents|4
  (params (Key :type Key%20Structure))
  (:Pressed
    (bind _outactors (Actor|GetAllActorsOfClass "/Game/Characters/BP_StagCharacter.BP_StagCharacter_C"))
    (if (> (Utilities|Array|Length _outactors) 0)
      (Pawn|Possess (Utilities|Array|Get(acopy) _outactors)))))

(event Input|KeyboardEvents|1
  (params (Key :type Key%20Structure))
  (:Pressed
    (bind _outactors (Actor|GetAllActorsOfClass "/Game/Characters/BP_FoxCharacter.BP_FoxCharacter_C"))
    (if (> (Utilities|Array|Length _outactors) 0)
      (Pawn|Possess (Utilities|Array|Get(acopy) _outactors)))))

(event Input|KeyboardEvents|2
  (params (Key :type Key%20Structure))
  (:Pressed
    (bind _outactors (Actor|GetAllActorsOfClass "/Game/Characters/BP_PigCharacter.BP_PigCharacter_C"))
    (if (> (Utilities|Array|Length _outactors) 0)
      (Pawn|Possess (Utilities|Array|Get(acopy) _outactors)))))

(event Input|KeyboardEvents|3
  (params (Key :type Key%20Structure))
  (:Pressed
    (bind _outactors (Actor|GetAllActorsOfClass "/Game/Characters/BP_DoeCharacter.BP_DoeCharacter_C"))
    (if (> (Utilities|Array|Length _outactors) 0)
      (Pawn|Possess (Utilities|Array|Get(acopy) _outactors)))))

(fn ConstructionScript)